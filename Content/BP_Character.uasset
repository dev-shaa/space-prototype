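; Player character that moves by push-off, with free pitch, yaw and roll camera control through Enhanced Input.
; Pushing sets the physics mesh's velocity along the camera's forward vector, allowed when forced, holding a handle, or when a sphere trace finds a surface behind and the cooldown has passed.
; Overlaps track the nearby BP_Handle, which the interact input grabs and releases; pushing also releases it.
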(event Input|EnhancedActionEvents|EnhancedInputActionIA_Interact
  (params (ActionValue :type Boolean) (ElapsedSeconds :type Float%20%28double-precision%29) (TriggeredSeconds :type Float%20%28double-precision%29) (InputAction :type Input%20Action%20Object%20Reference :default "/Game/IA_Interact.IA_Interact"))
  (:Started
    (if (Utilities|IsValid (Variables|Default|GetClose%20Handle))
      (bind _output_get (Variables|Default|SetCurrent%20Handle (Variables|Default|GetClose%20Handle)))
      (Default|Grab _output_get self)
      (Development|PrintString "Grabbed handle")))
  (:Canceled
    (CallFunction|ReleaseHandle :!label _label))
  (:Completed
    (goto _label)))

(event Input|EnhancedActionEvents|EnhancedInputActionIA_Push
  (params (ActionValue :type Boolean) (ElapsedSeconds :type Float%20%28double-precision%29) (TriggeredSeconds :type Float%20%28double-precision%29) (InputAction :type Input%20Action%20Object%20Reference :default "/Game/IA_Push.IA_Push"))
  (:Started
    (CallFunction|PushForward false)))

(event Input|EnhancedActionEvents|EnhancedInputActionIA_PitchYaw
  (params (ActionValue :type Vector%202D%20Structure) (ElapsedSeconds :type Float%20%28double-precision%29) (TriggeredSeconds :type Float%20%28double-precision%29) (InputAction :type Input%20Action%20Object%20Reference :default "/Game/IA_PitchYaw.IA_PitchYaw"))
  (bind (_x _y) (Math|Vector2D|BreakVector2D ActionValue))
  (Transformation|AddLocalRotation (Variables|Default|GetCamera) (Math|Rotator|MakeRotator 0.0 _y _x) false false))

(event Input|EnhancedActionEvents|EnhancedInputActionIA_Roll
  (params (ActionValue :type Float%20%28double-precision%29) (ElapsedSeconds :type Float%20%28double-precision%29) (TriggeredSeconds :type Float%20%28double-precision%29) (InputAction :type Input%20Action%20Object%20Reference :default "/Game/IA_Roll.IA_Roll"))
  (Transformation|AddLocalRotation (Variables|Default|GetCamera) (Math|Rotator|MakeRotator ActionValue 0.0 0.0) false false))

(event Collision|EventActorBeginOverlap
  (params (OtherActor :type Actor%20Object%20Reference))
  (bind _asbp_handle (Utilities|Casting|CastToBP_Handle OtherActor))
  (Variables|Default|SetClose%20Handle _asbp_handle)
  (Development|PrintString "Enter"))

(event Collision|EventActorEndOverlap
  (params (OtherActor :type Actor%20Object%20Reference))
  (if (== OtherActor (Variables|Default|GetClose%20Handle))
    (Variables|Default|SetClose%20Handle 0)
    (Development|PrintString "Exit")))

(event EventBeginPlay
  (bind _asplayer_controller (Utilities|Casting|CastToPlayerController (Pawn|GetController)))
  (Input|AddMappingContext (PlayerController|LocalPlayerSubsystems|GetEnhancedInputLocalPlayerSubsystem _asplayer_controller) "/Game/IMC_Custom.IMC_Custom" 0 "(bIgnoreAllPressedKeysUntilRelease=True,bForceImmediately=False,bNotifyUserSettings=False)"))

(fn ConstructionScript)

(fn HasSurfaceBehind
  (bind _returnvalue (Transformation|GetActorLocation))
  (bind _returnvalue_2 (Class|KismetSystemLibrary|SphereTraceSinglebyProfile _returnvalue (+ _returnvalue (* (Math|Vector|GetForwardVector (Variables|Default|GetCamera)) (Variables|Default|GetSurface%20Max%20Distance) -1.0)) 1e+01 "BlockAllDynamic" false 0 "None" true))
  (return _returnvalue_2))

(fn PushForward
  (params (Force :type Boolean))
  (if (Math|Boolean|ORBoolean Force (Utilities|IsValid (Variables|Default|GetCurrent%20Handle)) (and (CallFunction|HasSurfaceBehind) (CallFunction|CanPush)))
    (CallFunction|ReleaseHandle)
    (Physics|SetPhysicsLinearVelocity (Variables|Default|GetMesh) (* (Math|Vector|GetForwardVector (Variables|Default|GetCamera)) (Variables|Default|GetPush%20Velocity)) false "None")
    (Variables|Default|SetPush%20Time (Utilities|Time|GetRealTimeSeconds))
    (Development|PrintString "[Character] Pushed")))

(fn CanPush
  (return (>= (- (Utilities|Time|GetRealTimeSeconds) (Variables|Default|GetPush%20Time)) (Variables|Default|GetPush%20Delay))))

(fn ReleaseHandle
  (if (Utilities|IsValid (Variables|Default|GetCurrent%20Handle))
    (Default|Release (Variables|Default|GetCurrent%20Handle))
    (Variables|Default|SetCurrent%20Handle 0)
    (Development|PrintString "Released handle")))